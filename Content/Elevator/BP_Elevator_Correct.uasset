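; Elevator actor that travels between floors on call, with sliding doors, movement sounds and an arrival sound.
; CallElevator plays or reverses a timeline that samples a spline for cab height, stopping at the spline point matching the requested floor.
; A trigger box tracks the current BP_ElevatorFloorDoor_Correct, so floor and cab doors open together and close on a cooldown timer or before departure.
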(event `OpenElevatorDoors`
  (bind _doorleft (`self.DoorLeft`))
  (bind (_relativelocation_x _relativelocation_y _relativelocation_z) (`KismetMathLibrary.BreakVector` (`SceneComponent.RelativeLocation` _doorleft)))
  ;[1 1 1] Opening and closing elevator doors
  (if (not (`self.IsDoorOpened`))
    (set `self.IsDoorOpened` true)
    (bind (_direction _doordriver) (`Timeline|OpenDoorTimeline` :!label _label)
      (:`Update`
        (`SceneComponent.K2_SetRelativeLocation` _doorleft (`KismetMathLibrary.MakeVector` _doordriver _relativelocation_y _relativelocation_z) false false)
        (bind _result (`/Engine/EditorBlueprintResources/StandardMacros.NegateFloat` _doordriver)
          (:`  `
            (`SceneComponent.K2_SetRelativeLocation` (`self.DoorRight`) (`KismetMathLibrary.MakeVector` _result _relativelocation_y _relativelocation_z) false false)))))))

(event `CloseElevatorDoors`
  ;[1 1 1] Opening and closing elevator doors
  (if (`self.IsDoorOpened`)
    (set `self.IsDoorOpened` false)
    (goto _label :!via `Reverse`)))

(event `OpenDoors`
  ;[1 1 1] Opening and closing floor and lift doors
  (`self.OpenElevatorDoors`)
  (`/Game/Elevator/BP_ElevatorFloorDoor_Correct.OpenFloorDoor` (`self.CurrentFloorDoor`))
  (bind _returnvalue (`KismetSystemLibrary.K2_SetTimerDelegate` (delegate `CloseDoors`) (`self.ClosingCooldown`))))

(event `self.ReceiveTick`
  (params (DeltaSeconds :type "Float (single-precision)")))

(event `CloseDoors`
  ;[1 1 1] Opening and closing floor and lift doors
  (`|ExecutionSequence`
    (:`then_0`
      (`KismetSystemLibrary.K2_ClearAndInvalidateTimerHandle` (stale `OpenDoors` _returnvalue)))
    (:`then_1`
      (`self.CloseElevatorDoors`)
      (`/Game/Elevator/BP_ElevatorFloorDoor_Correct.CloseFloorDoor` (`self.CurrentFloorDoor`)))))

(event `CallElevator`
  (params (FloorNumber :type Integer))
  (bind _spline (`self.Spline`))
  (bind _spline_2 (`self.Spline`))
  (bind (_returnvalue_x _returnvalue_y _returnvalue_z) (`KismetMathLibrary.BreakVector` (`SplineComponent.GetLocationAtSplinePoint` _spline (`self.SelectedFloor`) "Local")))
  (bind (_returnvalue_x_2 _returnvalue_y_2 _returnvalue_z_2) (`KismetMathLibrary.BreakVector` (`SplineComponent.GetLocationAtSplinePoint` _spline_2 (`self.SelectedFloor`) "Local")))
  (if (not (`self.IsElevatorMoving`))
    (bind _result (`/Engine/EditorBlueprintResources/StandardMacros.DecrementInt` FloorNumber)
      (:`  `
        (bind _output_get (set `self.SelectedFloor` _result))
        (`/Engine/EditorBlueprintResources/StandardMacros.CompareInt` _output_get (`self.CurrentFloor`)
          (:`>`
            (set `self.IsElevatorMoving` true)
            (`self.CloseDoors`)
            (`KismetSystemLibrary.Delay` 1.0)
            (`AudioComponent.Play` (`self.MoveElevatorSound`) 0.0)
            (bind (_direction _elevatormodetrack) (`Timeline|MoveElevator` :!label _label_2)
              (:`Update`
                (switch `ETimelineDirection` _direction
                  (:`Forward`
                    (bind (_returnvalue_x_3 _returnvalue_y_3 _returnvalue_z_3) (`KismetMathLibrary.BreakVector` (`SplineComponent.GetLocationAtTime` _spline_2 _elevatormodetrack "Local" false)))
                    ;[1 1 1] Up Direction
                    (if (> _returnvalue_z_2 _returnvalue_z_3)
                      (`SceneComponent.K2_SetRelativeLocation` (`self.SM_Elevator`) (`KismetMathLibrary.MakeVector` 0.0 0.0 _returnvalue_z_3) false false)
                      (else
                        (set `self.CurrentFloor` (`self.SelectedFloor`))
                        (`self.OpenDoors` :!label _label_3)
                        (set `self.IsElevatorMoving` false)
                        (`AudioComponent.Stop` (`self.MoveElevatorSound`))
                        (`AudioComponent.Play` (`self.DoneElevatorSound`) 2.5)
                        (goto _label_2 :!via `Stop`))))
                  (:`Backward`
                    (bind (_returnvalue_x_4 _returnvalue_y_4 _returnvalue_z_4) (`KismetMathLibrary.BreakVector` (`SplineComponent.GetLocationAtTime` _spline _elevatormodetrack "Local" false)))
                    ;[1 1 1] Down direction
                    (if (< _returnvalue_z _returnvalue_z_4)
                      (`SceneComponent.K2_SetRelativeLocation` (`self.SM_Elevator`) (`KismetMathLibrary.MakeVector` 0.0 0.0 _returnvalue_z_4) false false)
                      (else
                        (set `self.CurrentFloor` (`self.SelectedFloor`))
                        (goto _label_3))))))))
          (:`==`
            (`self.OpenDoors`))
          (:`<`
            (set `self.IsElevatorMoving` true)
            (`self.CloseDoors`)
            (`KismetSystemLibrary.Delay` 1.0)
            (`AudioComponent.Play` (`self.MoveElevatorSound`) 0.0)
            (goto _label_2 :!via `Reverse`)))))))

(event `self.ReceiveActorBeginOverlap`
  (params (OtherActor :type "Actor Object Reference")))

(event `self.ReceiveBeginPlay`
  (`self.SetCurrentElevatorFloorDoors` (`|GetArrayItem` (`PrimitiveComponent.GetOverlappingActors` (`self.TriggerBox`) (`self.FloorDoorExampleActor`)))))

(event `self.TriggerBox.OnComponentBeginOverlap`
  (params (OverlappedComponent :type "PrimitiveComponent Object Reference") (OtherActor :type "Actor Object Reference") (OtherComp :type "PrimitiveComponent Object Reference") (OtherBodyIndex :type Integer) (bFromSweep :type Boolean) (SweepResult :type "HitResult Structure (by ref)"))
  (`self.SetCurrentElevatorFloorDoors` OtherActor))

(fn `SetCurrentElevatorFloorDoors`
  (params (FloorDoorActor :type "Actor Object Reference"))
  (if (== (`GameplayStatics.GetObjectClass` FloorDoorActor) (`self.FloorDoorExampleActor`))
    (bind _asbp_elevator_floor_door_correct (cast `/Game/Elevator/BP_ElevatorFloorDoor_Correct` FloorDoorActor))
    (set `self.CurrentFloorDoor` _asbp_elevator_floor_door_correct)))

(fn `UserConstructionScript`)