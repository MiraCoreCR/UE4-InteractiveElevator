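; Elevator floor door actor with two sliding panels that open and close through OpenFloorDoor and CloseFloorDoor events.
; An IsDoorOpen flag ignores redundant calls, and the DoorOpen timeline plays forward to open and reverses to close.
; Its DoorDriver track lerps each panel's relative X between closed and open coordinates, with the right panel derived from the left's value and height held fixed.
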(event `OpenFloorDoor`
  (if (not (`self.IsDoorOpen`))
    (set `self.IsDoorOpen` true)
    (bind (_direction _doordriver) (`Timeline|DoorOpen` :!label _label)
      (:`Update`
        (bind _returnvalue (`KismetMathLibrary.Lerp` (`self.ClosedDoorsCoordinate`) (`self.OpenDoorsCoordinate`) _doordriver))
        (`SceneComponent.K2_SetRelativeLocation` (`self.DoorLeft`) (`KismetMathLibrary.MakeVector` _returnvalue 0.0 150.0) false false)
        (bind _result (`/Engine/EditorBlueprintResources/StandardMacros.NegateFloat` _returnvalue)
          (:`  `
            (`SceneComponent.K2_SetRelativeLocation` (`self.DoorRight`) (`KismetMathLibrary.MakeVector` _result 0.0 150.0) false false)))))))

(event `CloseFloorDoor`
  (if (`self.IsDoorOpen`)
    (set `self.IsDoorOpen` false)
    (goto _label :!via `Reverse`)))

(event `self.ReceiveBeginPlay`)

(fn `UserConstructionScript`)