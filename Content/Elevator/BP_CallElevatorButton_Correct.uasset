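; Elevator call button actor that, on Interact, tells its target elevator Blueprint to travel to this button's floor number.
; Each press also plays a push sound and a timeline that slides the cylinder along Y.
; When NeedAttach is set, it snaps to a named socket on the elevator's mesh in both the construction script and BeginPlay, keeping world scale.
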(event `/Game/Elevator/IInteractible.Interact`
  (`/Game/Elevator/BP_Elevator_Correct.CallElevator` (`self.TargetElevatorBlueprint`) (`self.FloorNumber`))
  (`self.PlayCallElevatorButtonAnim`)
  (`AudioComponent.Play` (`self.PushButtonSound`) 0.0))

(event `PlayCallElevatorButtonAnim`
  (bind (_direction _pushbuttoncurve) (`Timeline|PushButton` :!via `PlayFromStart`)
    (:`Update`
      (`SceneComponent.K2_SetRelativeLocation` (`self.Cylinder`) (`KismetMathLibrary.MakeVector` 0.0 _pushbuttoncurve) false false))))

(event `self.ReceiveBeginPlay`
  (`self.AttachToElevatorSocket`))

(event `self.ReceiveTick`
  (params (DeltaSeconds :type "Float (single-precision)")))

(fn `AttachToElevatorSocket`
  (if (`self.NeedAttach`)
    (`self.K2_AttachToComponent` (`/Game/Elevator/BP_Elevator_Correct.SM_Elevator` (`self.TargetElevatorBlueprint`)) (`self.SocketName`) "SnapToTarget" "SnapToTarget" "KeepWorld" false)))

(fn `UserConstructionScript`
  (`self.AttachToElevatorSocket`))